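; AI controller for enemy goblins that investigates where the stealth character was perceived.
; On each perception update for a StealthCharacter that is not dead, it moves its pawn to the stimulus location, without checking whether the stimulus was gained or lost.
; On arrival, it sets the goblin's Searching flag and calls Roam, then clears the flag after a fixed delay.
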(event `self.AIPerception.OnTargetPerceptionUpdated`
  (params (Actor :type "Actor Object Reference") (Stimulus :type "AIStimulus Structure"))
  (bind _asstealth_character (cast `/Game/Blueprints/StealthCharacter` Actor))
  (if (not (`/Game/Blueprints/StealthCharacter.Dead` _asstealth_character))
    (`|AIMoveTo` (`self.K2_GetPawn`) (`.StimulusLocation` (break `AIStimulus` Stimulus)) null 50.0
      (:`OnSuccess`
        (bind _asenemy_goblin (cast `/Game/Blueprints/AI/EnemyGoblin` (`self.K2_GetPawn`)))
        (set `/Game/Blueprints/AI/EnemyGoblin.Searching` true _asenemy_goblin)
        (`/Game/Blueprints/AI/EnemyGoblin.roam` _asenemy_goblin)
        (`KismetSystemLibrary.Delay` 20.0)
        (set `/Game/Blueprints/AI/EnemyGoblin.Searching` false _asenemy_goblin)))))

(fn `UserConstructionScript`)