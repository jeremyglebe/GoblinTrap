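; Goblin enemy for a stealth game that patrols waypoints and kills any StealthCharacter entering its sphere.
; Patrol is a looping AI move that advances and wraps the waypoint index, pausing briefly at each point.
; The roam event moves it to random nearby reachable points while Searching is set, then shrugs and resumes patrol.
; A kill plays a sword-thrust montage, stops movement and flags KilledPlayer, which blocks further roaming.
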(event `self.ReceiveBeginPlay`
  (`self.Move Next Waypoint`))

(event `Move Next Waypoint`
  (`self.MoveToWaypoint`))

(event `roam`
  (`self.RandomRoam`))

(event `self.Sphere.OnComponentBeginOverlap`
  (params (OverlappedComponent :type "PrimitiveComponent Object Reference") (OtherActor :type "Actor Object Reference") (OtherComp :type "PrimitiveComponent Object Reference") (OtherBodyIndex :type Integer) (bFromSweep :type Boolean) (SweepResult :type "HitResult Structure (by ref)"))
  (bind _asstealth_character (cast `/Game/Blueprints/StealthCharacter` OtherActor))
  (`/Game/Blueprints/StealthCharacter.Die` _asstealth_character)
  (`|PlayMontage` (`self.Mesh`) "/Game/Blueprints/AI/AM_1H_sword_thrust_mid_Montage.AM_1H_sword_thrust_mid_Montage"
    (:`then`
      (set `self.KilledPlayer` true)
      (`NavMovementComponent.StopActiveMovement` (`self.CharacterMovement`)))))

(fn `UserConstructionScript`)