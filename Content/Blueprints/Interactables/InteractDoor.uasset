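; Interactable double door that swings open when activated, with a construction script that sets the prompt to "Unlock" if locked.
; Activate sets the Activated flag, plays the opening sound and starts a timeline roughly matched to the sound's length.
; The timeline yaws both leaves outward in opposite directions via FInterpTo, using elapsed timeline time as DeltaTime.
; On finish, it disables the box collision that blocks sight and navigation.
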(event `/Game/Blueprints/Interactables/InterfaceInteractable.Activate`
  (set `self.Activated` true)
  ;[1 1 1] Play door open sound
  (`GameplayStatics.PlaySoundAtLocation` "/Game/Audio/open_door.open_door" (`SceneComponent.K2_GetComponentLocation` (`self.SM_DoorWay`)) (struct) 1.0 1.0 0.0 null null null)
  ;[1 1 1] Animate opening the door
  (bind (_direction _time) (`Timeline|TimelineOpenDoor` :!via `PlayFromStart`) ; timline is approximate length of sound
    (:`Update`
      ;;[1 1 1] Open right door
      (`SceneComponent.K2_SetRelativeRotation` (`self.SM_DoorWay_Large_Door_Right`) (`KismetMathLibrary.MakeRotator` 0.0 0.0 (`KismetMathLibrary.FInterpTo` 0.0 -100.0 _time 1.0)) false false)
      ;;[1 1 1] Open left door
      (`SceneComponent.K2_SetRelativeRotation` (`self.SM_DoorWay_Large_Door_Left`) (`KismetMathLibrary.MakeRotator` 0.0 0.0 (`KismetMathLibrary.FInterpTo` 0.0 100.0 _time 1.0)) false false))
    (:`Finished`
      ;[1 1 1] Disable sight collision box and nav interruption
      (`PrimitiveComponent.SetCollisionEnabled` (`self.Box`) "NoCollision"))))

(fn `UserConstructionScript`
  (if (`self.Locked`)
    (set `self.Prompt` "Unlock"))
  (`parent.UserConstructionScript`))