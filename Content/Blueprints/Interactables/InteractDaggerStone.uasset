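; Interactable dagger stone that, when activated, slides its dagger mesh upward and then triggers a connected object.
; Activation sets a flag, plays the dagger sound and runs a timeline, timed to roughly match the sound, that drives the mesh height through FInterpTo.
; When the timeline finishes, it disables the sight collision box, drops the dagger with physics simulation and sends ActivateMessage to ConnectedTo.
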(event `/Game/Blueprints/Interactables/InterfaceInteractable.Activate`
  (set `self.Activated` true)
  ;[1 1 1] Play sound
  (`GameplayStatics.PlaySoundAtLocation` "/Game/Audio/dagger.dagger" (`SceneComponent.K2_GetComponentLocation` (`self.SM_Dagger_01b`)) (struct) 1.0 1.0 0.0 null null null)
  ;[1 1 1] Animate opening the door
  (bind (_direction _time) (`Timeline|Timeline_0`) ; timline is approximate length of sound
    (:`Update`
      (`SceneComponent.K2_SetRelativeLocation` (`self.SM_Dagger_01b`) (`KismetMathLibrary.MakeVector` -5.0 -5.0 (`KismetMathLibrary.FInterpTo` 60.0 110.0 _time 1.0)) false false))
    (:`Finished`
      ;[1 1 1] Disable sight collision box
      (`PrimitiveComponent.SetCollisionEnabled` (`self.Box`) "NoCollision")
      ;[1 1 1] Drop the dagger
      (`PrimitiveComponent.SetSimulatePhysics` (`self.SM_Dagger_01b`) true)
      (message `/Game/Blueprints/Triggerable/ITriggerable.Activate` (`self.ConnectedTo`)))))

(fn `UserConstructionScript`
  (`parent.UserConstructionScript`))