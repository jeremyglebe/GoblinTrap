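; InteractChest is an interactable chest that opens its lid when activated.
; The Activate event sets Activated, plays a sound at the lid and starts a timeline that rolls the lid open.
; The timeline's Time track feeds FInterpTo as its delta time to drive the rotation.
; When the timeline finishes, the Box component's collision is disabled, commented as clearing sight blocking and nav interruption.
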(event `/Game/Blueprints/Interactables/InterfaceInteractable.Activate`
  (set `self.Activated` true)
  ;[1 1 1] Play door open sound
  (`GameplayStatics.PlaySoundAtLocation` "/Game/Audio/open_door.open_door" (`SceneComponent.K2_GetComponentLocation` (`self.Lid`)) (struct) 1.0 1.0 0.0 null null null)
  ;[1 1 1] Animate opening the door
  (bind (_direction _time) (`Timeline|Timeline_1` :!via `PlayFromStart`)
    (:`Update`
      ;;[1 1 1] Open right door
      (`SceneComponent.K2_SetRelativeRotation` (`self.Lid`) (`KismetMathLibrary.MakeRotator` (`KismetMathLibrary.FInterpTo` 0.0 -100.0 _time 1.0)) false false))
    (:`Finished`
      ;[1 1 1] Disable sight collision box and nav interruption
      (`PrimitiveComponent.SetCollisionEnabled` (`self.Box`) "NoCollision"))))

(fn `UserConstructionScript`
  (`parent.UserConstructionScript`))