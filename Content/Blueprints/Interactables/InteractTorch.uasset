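; InteractTorch is an interactable torch that lights up when activated.
; Its Activate event shows the point light and fire particle, then sets the Lit and Activated flags.
; The construction script runs the parent's, then matches light and fire visibility to Lit so the torch can start lit or unlit.
; Activation only lights the torch; nothing here extinguishes it.
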(event `/Game/Blueprints/Interactables/InterfaceInteractable.Activate`
  (`SceneComponent.SetVisibility` (`self.Torch_PointLight`) true false)
  (`SceneComponent.SetVisibility` (`self.P_Torch_Fire`) true false)
  (set `self.Lit` true)
  (set `self.Activated` true))

(fn `UserConstructionScript`
  (bind _p_torch_fire (`self.P_Torch_Fire`))
  (bind _torch_pointlight (`self.Torch_PointLight`))
  (`parent.UserConstructionScript`)
  (if (`self.Lit`)
    (`SceneComponent.SetVisibility` _torch_pointlight true false)
    (`SceneComponent.SetVisibility` _p_torch_fire true false)
    (else
      (`SceneComponent.SetVisibility` _torch_pointlight false false)
      (`SceneComponent.SetVisibility` _p_torch_fire false false))))